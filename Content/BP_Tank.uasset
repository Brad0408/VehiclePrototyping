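; BP_Tank is a drivable tank pawn built on Chaos wheeled vehicle movement.
; Enhanced Input actions feed steering as yaw, throttle and brake to the movement component, while look input yaws the spring arm camera.
; A legacy MouseY axis event sets vehicle pitch input.
; Each tick fakes track motion by driving the mesh materials' OffsetV parameter from scaled forward speed.
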(event `self.ReceiveBeginPlay`
  (bind _aschaos_wheeled_vehicle_movement_component (cast `ChaosWheeledVehicleMovementComponent` (`self.VehicleMovementComponent`)))
  (set `self.Chaos Wheeled Vehicle Movement Component` _aschaos_wheeled_vehicle_movement_component))

(event `EnhancedInput|/Game/VehicleTemplate/Input/Actions/IA_LookAround`
  (params (ActionValue :type "Float (double-precision)") (ElapsedSeconds :type "Float (double-precision)") (TriggeredSeconds :type "Float (double-precision)") (InputAction :type "InputAction Object Reference" :default "/Game/VehicleTemplate/Input/Actions/IA_LookAround.IA_LookAround"))
  (:`Triggered`
    (`SceneComponent.K2_AddLocalRotation` (`self.SpringArm`) (`KismetMathLibrary.MakeRotator` 0.0 0.0 ActionValue) false false) ; Rotate camera around the vehicle
  ))

(event `InputAxisKey|MouseY`
  (params (AxisValue :type "Float (single-precision)"))
  (`ChaosVehicleMovementComponent.SetPitchInput` (`self.ChaosWheeledVehicleMovement`) AxisValue))

(event `EnhancedInput|/Game/VehicleTemplate/Input/Actions/IA_Steering`
  (params (ActionValue :type "Float (double-precision)") (ElapsedSeconds :type "Float (double-precision)") (TriggeredSeconds :type "Float (double-precision)") (InputAction :type "InputAction Object Reference" :default "/Game/VehicleTemplate/Input/Actions/IA_Steering.IA_Steering"))
  (:`Triggered`
    (`ChaosVehicleMovementComponent.SetYawInput` (`self.ChaosWheeledVehicleMovement`) ActionValue :!label _label))
  (:`Completed`
    (goto _label)))

(event `EnhancedInput|/Game/VehicleTemplate/Input/Actions/IA_Throttle`
  (params (ActionValue :type "Float (double-precision)") (ElapsedSeconds :type "Float (double-precision)") (TriggeredSeconds :type "Float (double-precision)") (InputAction :type "InputAction Object Reference" :default "/Game/VehicleTemplate/Input/Actions/IA_Throttle.IA_Throttle"))
  (:`Triggered`
    (`ChaosVehicleMovementComponent.SetThrottleInput` (`self.ChaosWheeledVehicleMovement`) ActionValue :!label _label_2))
  (:`Completed`
    (goto _label_2)))

(event `EnhancedInput|/Game/VehicleTemplate/Input/Actions/IA_Break`
  (params (ActionValue :type "Float (double-precision)") (ElapsedSeconds :type "Float (double-precision)") (TriggeredSeconds :type "Float (double-precision)") (InputAction :type "InputAction Object Reference" :default "/Game/VehicleTemplate/Input/Actions/IA_Break.IA_Break"))
  (:`Triggered`
    (`ChaosVehicleMovementComponent.SetBrakeInput` (`self.ChaosWheeledVehicleMovement`) ActionValue :!label _label_3))
  (:`Completed`
    (goto _label_3)))

(event `self.ReceiveTick`
  (params (DeltaSeconds :type "Float (single-precision)"))
  (`self.TrackAnimations`))

(event `TrackAnimations`
  (`MeshComponent.SetScalarParameterValueOnMaterials` (`self.Mesh`) "OffsetV" (* (`ChaosVehicleMovementComponent.GetForwardSpeedMPH` (`self.ChaosWheeledVehicleMovement`)) 0.75)))

(fn `UserConstructionScript`)