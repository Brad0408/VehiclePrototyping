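; BP_Room is a room actor that sets its own layout mesh and populates it with doors at BeginPlay.
; A spawn room uses SM_Spawn, while any other room picks randomly between SM_Cross and SM_Long.
; It then spawns a BP_Door at the world transform of every socket on the chosen mesh, so the mesh sockets define door placement.
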(event `self.ReceiveBeginPlay`
  (`StaticMeshComponent.SetStaticMesh` (`self.Room`) (select `bool` (`self.IsSpawnRoom`) :`false` (`KismetArrayLibrary.Array_Random` (`|MakeArray` "/Game/VehicleTemplate/Maps/_GENERATED/c011185l/SM_Cross.SM_Cross" "/Game/VehicleTemplate/Maps/_GENERATED/c011185l/SM_Long.SM_Long" :!type "StaticMesh Object Reference")) :`true` "/Game/VehicleTemplate/Maps/_GENERATED/c011185l/SM_Spawn.SM_Spawn"))
  (for _array_element (`SceneComponent.GetAllSocketNames` (`self.Room`))
    (`|SpawnActorFromClass` "/Game/BP/PG/BP_Door.BP_Door_C" (`SceneComponent.GetSocketTransform` (`self.Room`) _array_element "RTS_World") "Undefined" "MultiplyWithRoot" null null)))

(fn `UserConstructionScript`)