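; BP_ActorGenerator is an actor that populates a spline with BP_Spawnable actors when play begins.
; On BeginPlay it divides the spline length by the Distance spacing, rounds the result, and spawns one actor at each step, including the start point.
; Each spawn takes only its world-space location from the spline, not its rotation.
; The construction script is empty, so nothing is generated in the editor.
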(event `self.ReceiveBeginPlay`
  (for _index (range (+ (`KismetMathLibrary.Round` (/ (`SplineComponent.GetSplineLength` (`self.Spline`)) (`self.Distance`))) 1))
    (`|SpawnActorFromClass` "/Game/BP/Spline/BP_Spawnable.BP_Spawnable_C" (`KismetMathLibrary.MakeTransform` (`SplineComponent.GetLocationAtDistanceAlongSpline` (`self.Spline`) (* _index (`self.Distance`)) "World")) "Undefined" "MultiplyWithRoot" null null)))

(fn `UserConstructionScript`)