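; Breakable Chaos geometry collection actor that fades and removes itself some time after being hit.
; The construction script sets the rest collection from ObjectToBreak, so one Blueprint serves different breakable meshes.
; A component hit starts a delay, then swaps both material slots to a faded wall or transparent pillar material, depending on whether the collection is the castle wall.
; A second delay then destroys the actor.
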(event `self.GeometryCollection.OnComponentHit`
  (params (HitComponent :type "PrimitiveComponent Object Reference") (OtherActor :type "Actor Object Reference") (OtherComp :type "PrimitiveComponent Object Reference") (NormalImpulse :type "Vector Structure") (Hit :type "HitResult Structure (by ref)"))
  (`KismetSystemLibrary.Delay` 20.0)
  (for _index (range 2)
    (if (== (`self.ObjectToBreak`) "/Game/DestructibleEnvrionement/S_Castle_Wall_sebgb_lod5_GeometryCollection.S_Castle_Wall_sebgb_lod5_GeometryCollection")
      (`PrimitiveComponent.SetMaterial` (`self.GeometryCollection`) _index "/Game/Megascans/3D_Assets/Castle_Wall_sebgb/M_FadedWall.M_FadedWall")
      (`KismetSystemLibrary.Delay` 10.0)
      (`self.K2_DestroyActor`)
      (else
        (`PrimitiveComponent.SetMaterial` (`self.GeometryCollection`) _index "/Game/Megascans/3D_Assets/Castle_Column_scohv/M_PillarTransparent.M_PillarTransparent")
        (`KismetSystemLibrary.Delay` 10.0)
        (`self.K2_DestroyActor`)))))

(fn `UserConstructionScript`
  (`GeometryCollectionComponent.SetRestCollection` (`self.GeometryCollection`) (`self.ObjectToBreak`)))