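; BP_TankShell is a tank shell projectile that explodes where its movement component stops on impact.
; On stop it spawns and triggers an FS_MasterField at the impact point, then plays a Niagara explosion and attenuated sound.
; It applies radial damage with falloff and a velocity-change radial impulse to the hit component only, then destroys itself.
; A debug sphere for the inner damage radius is left disconnected.
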(event `self.ProjectileMovement.OnProjectileStop`
  (params (ImpactResult :type "HitResult Structure (by ref)"))
  (bind (_bblockinghit _binitialoverlap _time _distance _location _impactpoint _normal _impactnormal _physmat _hitactor _hitcomponent) (`GameplayStatics.BreakHitResult` ImpactResult))
  (bind _returnvalue (`|SpawnActorFromClass` "/Engine/EditorResources/FieldNodes/FS_MasterField.FS_MasterField_C" (`KismetMathLibrary.MakeTransform` _impactpoint) "Undefined" "MultiplyWithRoot" null null))
  (set `/Engine/EditorResources/FieldNodes/FS_MasterField.ActivationType` "NewEnumerator4" _returnvalue)
  (`/Engine/EditorResources/FieldNodes/FS_MasterField.CE_Trigger` _returnvalue)
  (`NiagaraFunctionLibrary.SpawnSystemAtLocation` "/Game/VigilanteMovement/Shared/Particles/NiagaraSystems/NS_OrdinanceExplosion.NS_OrdinanceExplosion" _location (`KismetMathLibrary.MakeRotFromZ` _impactnormal)) ; Spawn explosion VFX at impact point
  (`GameplayStatics.SpawnSoundAtLocation` "/Game/SFX/ES_Grenade_Explosion_14_-_SFX_Producer.ES_Grenade_Explosion_14_-_SFX_Producer" _location (struct) 1.0 1.0 0.0 "/Game/SFX/ATT_TankShell.ATT_TankShell" null) ; Spawn SFX at impact point
  (`GameplayStatics.ApplyRadialDamageWithFalloff` :`BaseDamage` (`self.Base Damage`) :`MinimumDamage` (`self.Minimum Damage`) :`Origin` _impactpoint :`DamageInnerRadius` (`self.Damage Inner Radius`) :`DamageOuterRadius` (`self.Damage Outer Radius`) :`DamageFalloff` 1.0 :`DamageCauser` null :`InstigatedByController` null) ; Apply radial damage at impact point
  (`/Engine/EditorBlueprintResources/StandardMacros.IsValid` _hitcomponent
    (:`Is Valid`
      (`PrimitiveComponent.AddRadialImpulse` _hitcomponent _impactpoint (`self.Damage Outer Radius`) 1500.0 "RIF_Constant" true) ; Add radial impulse at impact point, make things move whn hit
      (`self.K2_DestroyActor`))
    (:`Is Not Valid`
      (`self.K2_DestroyActor`))))

(fn `UserConstructionScript`)