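; BP_TankDecoy is a destructible decoy tank that takes damage and turns into a wreck.
; AnyDamage feeds ModifyHealth, which subtracts damage from Health only while Health is above zero.
; When Health drops to zero or below, it spawns an ordinance explosion Niagara effect, destroys itself and spawns BP_DestroyedTank at its transform.
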(event `self.ReceiveAnyDamage`
  (params (Damage :type "Float (single-precision)") (DamageType :type "DamageType Object Reference") (InstigatedBy :type "Controller Object Reference") (DamageCauser :type "Actor Object Reference"))
  (`self.ModifyHealth` Damage))

(fn `ModifyHealth`
  (params (Damage :type "Float (double-precision)"))
  (bind _returnvalue (`self.GetTransform`))
  (if (> (`self.Health`) 0.0)
    (bind _output_get (set `self.Health` (- (`self.Health`) Damage)))
    (if (<= _output_get 0.0)
      (`NiagaraFunctionLibrary.SpawnSystemAtLocation` "/Game/VigilanteMovement/Shared/Particles/NiagaraSystems/NS_OrdinanceExplosion.NS_OrdinanceExplosion" (.location _returnvalue) (.rotation _returnvalue))
      (`self.K2_DestroyActor`)
      (`|SpawnActorFromClass` "/Game/Tank/BP_DestroyedTank.BP_DestroyedTank_C" _returnvalue "AlwaysSpawn" "MultiplyWithRoot" null null))))

(fn `UserConstructionScript`)