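; Player tank on Chaos vehicle movement that creates health, reload and crosshair widgets and toggles a pause menu.
; Tick derives Reversing from wheel spin to drive track audio.
; Damage feeds ModifyHealth, which swaps in a wreck and respawn screen at zero health.
; Shooting plays a recoil timeline with reload delay, but shell spawning, camera, steering, speed-limit, dust, decal, engine-sound and track-animation logic is disconnected.
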(event `self.ReceiveBeginPlay`
  ;[1 1 1] BeginCasts
  (set `self.As GI Data` (cast `/Game/GI_Data` (`GameplayStatics.GetGameInstance`) :!pure true))
  (`self.GetUIElements`)
  (bind _aschaos_wheeled_vehicle_movement_component (cast `ChaosWheeledVehicleMovementComponent` (`self.VehicleMovementComponent`)))
  (set `self.Chaos Wheeled Vehicle Movement Component` _aschaos_wheeled_vehicle_movement_component)
  (bind _asvehicle_player_controller (cast `/Game/VehicleTemplate/Blueprints/VehiclePlayerController` (`GameplayStatics.GetPlayerController` 0)))
  (set `self.PlayerController` _asvehicle_player_controller))

(event `SetMaxSpeed`
  ;[1 1 1] Speed Limits
)

(event `self.ReceiveAnyDamage`
  (params (Damage :type "Float (single-precision)") (DamageType :type "DamageType Object Reference") (InstigatedBy :type "Controller Object Reference") (DamageCauser :type "Actor Object Reference"))
  ;[1 1 1] Damage
  (`self.ModifyHealth` Damage :!label _label))

(event `self.ReceiveRadialDamage`
  (params (DamageReceived :type "Float (single-precision)") (DamageType :type "DamageType Object Reference") (Origin :type "Vector Structure") (HitInfo :type "HitResult Structure (by ref)") (InstigatedBy :type "Controller Object Reference") (DamageCauser :type "Actor Object Reference"))
  ;[1 1 1] Damage
  (goto _label))

(event `GetUIElements`
  ;[1 1 1] UI
  (bind _returnvalue (`|CreateWidget` "/Game/Widgets/W_HealthAndReload.W_HealthAndReload_C"))
  (bind _output_get (set `self.HealthUIRef` _returnvalue))
  (`UserWidget.AddToViewport` _output_get 0)
  (bind _returnvalue_2 (`|CreateWidget` "/Game/Widgets/W_Crosshair.W_Crosshair_C"))
  (bind _output_get_2 (set `self.CrosshairRef` _returnvalue_2))
  (`UserWidget.AddToViewport` _output_get_2 0))

(event `SetMaxReverse`
  ;[1 1 1] Speed Limits
)

(event `self.ReceiveTick`
  (params (DeltaSeconds :type "Float (single-precision)"))
  ;[1 1 1] Updating
  (if (> (`ChaosVehicleWheel.GetRotationAngularVelocity` (`|GetArrayItem` (`ChaosWheeledVehicleMovementComponent.Wheels` (`self.VehicleMoveComponent`)) 4)) 100.0)
    (set `self.Reversing?` true)
    (`self.SettingWheelDustLocaiton`)
    (`self.DecalTracks`)
    (`self.BPEngineSounds`)
    (`self.TankTrackSounds`)
    (else
      (set `self.Reversing?` false)
      (`self.SettingWheelDustLocaiton`)
      (`self.DecalTracks`)
      (`self.BPEngineSounds`)
      (`self.TankTrackSounds`))))

(event `EnhancedInput|/Game/VehicleTemplate/Input/Actions/IA_Steering`
  (params (ActionValue :type "Float (double-precision)") (ElapsedSeconds :type "Float (double-precision)") (TriggeredSeconds :type "Float (double-precision)") (InputAction :type "InputAction Object Reference" :default "/Game/VehicleTemplate/Input/Actions/IA_Steering.IA_Steering"))
  ;[0.05237 0.4734 1] Player INputs
  ;;[0.0565 0.2466 0.6667] Steering
)

(event `EnhancedInput|/Game/VehicleTemplate/Input/Actions/IA_LookAround`
  (params (ActionValue :type "Float (double-precision)") (ElapsedSeconds :type "Float (double-precision)") (TriggeredSeconds :type "Float (double-precision)") (InputAction :type "InputAction Object Reference" :default "/Game/VehicleTemplate/Input/Actions/IA_LookAround.IA_LookAround"))
  ;[0.05237 0.4734 1] Player INputs
  ;;[0.0565 0.2466 0.6667] Camera controlls
)

(event `TankTrackSounds`
  (bind _tank_tracks_cue (`self.Tank_Tracks_Cue`))
  (bind _tank_tracks_cue_2 (`self.Tank_Tracks_Cue`))
  (bind _returnvalue (`ChaosVehicleMovementComponent.GetForwardSpeedMPH` (`self.VehicleMoveComponent`)))
  (bind _returnvalue_2 (* (`ChaosVehicleMovementComponent.GetForwardSpeedMPH` (`self.VehicleMoveComponent`)) -1.0))
  ;[0.3537 0.02728 1] Visual and sounds tank changes
  ;;[0.6115 0.2022 0.8958] TankTrackSounds
  (if (`self.Reversing?`)
    (`AudioComponent.SetFloatParameter` _tank_tracks_cue_2 "Speed" _returnvalue_2)
    (`AudioComponent.SetVolumeMultiplier` _tank_tracks_cue_2 (`KismetMathLibrary.MapRangeClamped` _returnvalue_2 0.0 10.0 0.0 1.0))
    (else
      (`AudioComponent.SetFloatParameter` _tank_tracks_cue "Speed" _returnvalue)
      (`AudioComponent.SetVolumeMultiplier` _tank_tracks_cue (`KismetMathLibrary.MapRangeClamped` _returnvalue 0.0 10.0 0.0 1.0)))))

(event `SettingWheelDustLocaiton`
  ;[0.3537 0.02728 1] Visual and sounds tank changes
  ;;[0.6115 0.2022 0.8958] MOve Dust to front or back of tank
)

(event `EnhancedInput|/Game/NewIA/IA_LookUpAndDown`
  (params (ActionValue :type "Float (double-precision)") (ElapsedSeconds :type "Float (double-precision)") (TriggeredSeconds :type "Float (double-precision)") (InputAction :type "InputAction Object Reference" :default "/Game/NewIA/IA_LookUpAndDown.IA_LookUpAndDown"))
  ;[0.05237 0.4734 1] Player INputs
  ;;[0.0565 0.2466 0.6667] Camera controlls
)

(event `EnhancedInput|/Game/NewIA/IA_ScrollOut`
  (params (ActionValue :type "Float (double-precision)") (ElapsedSeconds :type "Float (double-precision)") (TriggeredSeconds :type "Float (double-precision)") (InputAction :type "InputAction Object Reference" :default "/Game/NewIA/IA_ScrollOut.IA_ScrollOut"))
  ;[0.05237 0.4734 1] Player INputs
  ;;[0.0565 0.2466 0.6667] Scroll in and out
)

(event `EnhancedInput|/Game/VehicleTemplate/Input/Actions/IA_Throttle`
  (params (ActionValue :type "Float (double-precision)") (ElapsedSeconds :type "Float (double-precision)") (TriggeredSeconds :type "Float (double-precision)") (InputAction :type "InputAction Object Reference" :default "/Game/VehicleTemplate/Input/Actions/IA_Throttle.IA_Throttle"))
  ;[0.05237 0.4734 1] Player INputs
  ;;[0.0565 0.2466 0.6667] Throttle and break
  (:`Triggered`
    (`self.DustEffects` :!label _label_2)
    (`self.SetMaxSpeed`)
    (`PlayerController.K2_ClientPlayForceFeedback` (`GameplayStatics.GetPlayerController` 0) "/Game/ControllerFeedback/FF_MovementRumble.FF_MovementRumble" "None" false false false))
  (:`Completed`
    (goto _label_2)))

(event `EnhancedInput|/Game/VehicleTemplate/Input/Actions/IA_Break`
  (params (ActionValue :type "Float (double-precision)") (ElapsedSeconds :type "Float (double-precision)") (TriggeredSeconds :type "Float (double-precision)") (InputAction :type "InputAction Object Reference" :default "/Game/VehicleTemplate/Input/Actions/IA_Break.IA_Break"))
  ;[0.05237 0.4734 1] Player INputs
  ;;[0.0565 0.2466 0.6667] Throttle and break
  (:`Triggered`
    (`self.SetMaxReverse` :!label _label_3)
    (`PlayerController.K2_ClientPlayForceFeedback` (`GameplayStatics.GetPlayerController` 0) "/Game/ControllerFeedback/FF_MovementRumble.FF_MovementRumble" "None" false false false))
  (:`Completed`
    (goto _label_3)))

(event `EnhancedInput|/Game/NewIA/IA_ScrollIn`
  (params (ActionValue :type "Float (double-precision)") (ElapsedSeconds :type "Float (double-precision)") (TriggeredSeconds :type "Float (double-precision)") (InputAction :type "InputAction Object Reference" :default "/Game/NewIA/IA_ScrollIn.IA_ScrollIn"))
  ;[0.05237 0.4734 1] Player INputs
  ;;[0.0565 0.2466 0.6667] Scroll in and out
)

(event `BPTrackAnimations`
  ;[0.3537 0.02728 1] Visual and sounds tank changes
  ;;[0.6115 0.2022 0.8958] Make track move by offeseting texture
)

(event `DecalTracks`
  ;[0.3537 0.02728 1] Visual and sounds tank changes
  ;;[0.6115 0.2022 0.8958] Spawn track decals at both tracks locations
)

(event `DustEffects`
  ;[0.3537 0.02728 1] Visual and sounds tank changes
  ;;[0.6115 0.2022 0.8958] Make dust appear when tank is moving and change size based of speed
)

(event `EnhancedInput|/Game/VehicleTemplate/Input/Actions/IA_ToggleCamera`
  (params (ActionValue :type Boolean) (ElapsedSeconds :type "Float (double-precision)") (TriggeredSeconds :type "Float (double-precision)") (InputAction :type "InputAction Object Reference" :default "/Game/VehicleTemplate/Input/Actions/IA_ToggleCamera.IA_ToggleCamera"))
  ;[0.05237 0.4734 1] Player INputs
  ;;[0.0565 0.2466 0.6667] First person mode
)

(event `EnhancedInput|/Game/NewIA/IA_Pause`
  (params (ActionValue :type Boolean) (ElapsedSeconds :type "Float (double-precision)") (TriggeredSeconds :type "Float (double-precision)") (InputAction :type "InputAction Object Reference" :default "/Game/NewIA/IA_Pause.IA_Pause"))
  (bind _pausemenuref (`self.PauseMenuRef`))
  ;[0.05237 0.4734 1] Player INputs
  ;;[0.0565 0.2466 0.6667] Pausing
  (:`Started`
    (`/Engine/EditorBlueprintResources/StandardMacros.IsValid` _pausemenuref
      (:`Is Valid`
        (`/Game/Widgets/W_PauseMenu.ContinueFake` _pausemenuref)
        (set `self.PauseMenuRef` null))
      (:`Is Not Valid`
        (bind _returnvalue (`|CreateWidget` "/Game/Widgets/W_PauseMenu.W_PauseMenu_C"))
        (bind _output_get (set `self.PauseMenuRef` _returnvalue))
        (`UserWidget.AddToViewport` _output_get 0)
        (set `PlayerController.bShowMouseCursor` true (`GameplayStatics.GetPlayerController` 0))))))

(event `EnhancedInput|/Game/NewIA/IA_Shoot`
  (params (ActionValue :type Boolean) (ElapsedSeconds :type "Float (double-precision)") (TriggeredSeconds :type "Float (double-precision)") (InputAction :type "InputAction Object Reference" :default "/Game/NewIA/IA_Shoot.IA_Shoot"))
  ;[0.05237 0.4734 1] Player INputs
  ;;[0.0565 0.2466 0.6667] Shotting
  (:`Triggered`
    (if (`self.bTankFired`)
      (bind (_direction _newtrack_0) (`Timeline|Recoil` :!via `PlayFromStart`)
        (:`Update`
          (set `self.RecoilAlpha` _newtrack_0)
          (set `self.bTankFired` false))
        (:`Finished`
          (`/Game/Widgets/W_HealthAndReload.UpdateReload` (`self.HealthUIRef`))
          (`KismetSystemLibrary.Delay` 1.2)
          (set `self.bTankFired` true))))))

(event `BPEngineSounds`
  ;[0.3537 0.02728 1] Visual and sounds tank changes
  ;;[0.6115 0.2022 0.8958] engine sounds
)

(fn `ModifyHealth`
  (params (Damage :type "Float (double-precision)"))
  (bind _returnvalue (`self.GetTransform`))
  (bind _playercontroller (`self.PlayerController`))
  (if (> (`self.Health`) 0.0)
    (bind _output_get (set `self.Health` (- (`self.Health`) Damage)))
    (`/Game/Widgets/W_HealthAndReload.UpdateHealth` (`self.HealthUIRef`) _output_get)
    (if (<= _output_get 0.0)
      (`NiagaraFunctionLibrary.SpawnSystemAtLocation` "/Game/VigilanteMovement/Shared/Particles/NiagaraSystems/NS_OrdinanceExplosion.NS_OrdinanceExplosion" (.location _returnvalue) (.rotation _returnvalue))
      (`self.K2_DestroyActor`)
      (`|SpawnActorFromClass` "/Game/Tank/BP_DestroyedTank.BP_DestroyedTank_C" _returnvalue "AlwaysSpawn" "MultiplyWithRoot" null null)
      ;[1 1 1] UI Updates
      (set `/Game/VehicleTemplate/Blueprints/VehiclePlayerController.TankRef` null _playercontroller)
      (`Widget.RemoveFromParent` (`/Game/VehicleTemplate/Blueprints/VehiclePlayerController.VehicleHud` _playercontroller))
      (`Widget.RemoveFromParent` (`self.CrosshairRef`))
      (bind _returnvalue_2 (`|CreateWidget` "/Game/Widgets/W_Respawn.W_Respawn_C"))
      (bind _output_get_2 (set `self.RespawUIRef` _returnvalue_2))
      (`UserWidget.AddToViewport` _output_get_2 0)
      (set `PlayerController.bShowMouseCursor` true (`GameplayStatics.GetPlayerController` 0)))))

(fn `UserConstructionScript`)